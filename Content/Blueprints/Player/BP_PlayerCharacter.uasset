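; Player character Blueprint with first-person style movement, look, jump and weapon fire input.
; On possession, the server has BPWeaponManager create and select an auto rifle, under a section labeled as a test.
; Fire press and release go through a client-to-server event that starts or stops the current weapon.
; GetVisibleMesh returns the hands mesh when locally controlled and the body mesh otherwise.
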(event Custom|Server_Fire
  (params (Activate :type Boolean))
  (bind _bp_weaponmanager (Variables|Default|GetBP_WeaponManager))
  (bind _currentweapon (Variables|/Game/Blueprints/Components/Player/BP_WeaponManager.BP_WeaponManager_C|GetCurrentWeapon _bp_weaponmanager))
  ;[1 1 1] Стрельба
  (if Activate
    (Default|UseWeapon _currentweapon)
    (else
      (Default|StopUseWeapon _currentweapon))))

(event EventPossessed
  (params (NewController :type Controller%20Object%20Reference))
  ;[1 1 1] Тест
  (Networking|SwitchHasAuthority
    (:Authority
      (bind _weapon (Default|CreateWeapon (Variables|Default|GetBP_WeaponManager) "/Game/Blueprints/Weapons/BP_Weapon_AutoRifles.BP_Weapon_AutoRifles_C"))
      (Default|SelectWeapon (Variables|Default|GetBP_WeaponManager) _weapon))))

(event Input|ActionEvents|InputActionFire
  (params (Key :type Key%20Structure :default "None"))
  ;[1 1 1] Стрельба
  (:Pressed
    (CallFunction|ServerFire true))
  (:Released
    (CallFunction|ServerFire false)))

(event Input|ActionEvents|InputActionJump
  (params (Key :type Key%20Structure :default "None"))
  ;[0.1639 0.174 1] Перемешение
  (:Pressed
    (Character|Jump)))

(event Input|AxisEvents|InputAxisLookUp
  (params (AxisValue :type Float%20%28single-precision%29))
  ;[0.1639 0.174 1] Перемешение
  (Pawn|Input|AddControllerPitchInput AxisValue))

(event Input|AxisEvents|InputAxisTurn
  (params (AxisValue :type Float%20%28single-precision%29))
  ;[0.1639 0.174 1] Перемешение
  (Pawn|Input|AddControllerYawInput AxisValue))

(event Input|AxisEvents|InputAxisMoveForward
  (params (AxisValue :type Float%20%28single-precision%29))
  ;[0.1639 0.174 1] Перемешение
  (Pawn|Input|AddMovementInput (Transformation|GetActorForwardVector) AxisValue false))

(event Input|AxisEvents|InputAxisMoveRight
  (params (AxisValue :type Float%20%28single-precision%29))
  ;[0.1639 0.174 1] Перемешение
  (Pawn|Input|AddMovementInput (Transformation|GetActorRightVector) AxisValue false))

(fn ConstructionScript)

(fn GetVisibleMesh
  (return (select (Pawn|IsLocallyControlled) (Variables|Default|GetHandsMash) (Variables|Character|GetMesh))))