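; Base HUD class that switches gameplay, spectate and tab widgets on round and player life events.
; It binds to game state round start/end, then to player state alive/dead on round start.
; The gameplay widget is created lazily and shown only while alive; death passes killer info to the spectate widget.
; Spectate and tab toggles ignore their Show input through hardcoded false branches, so they only remove widgets during active rounds.
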(event Custom|OnRoundStarted
  (bind _returnvalue (Game|Player|GetOwningPlayerController))
  (bind _playerstate (Variables|/Script/Engine.Controller|GetPlayerState _returnvalue))
  (bind _asbp_player_state (Utilities|Casting|CastToBP_PlayerState _playerstate))
  (CallFunction|ToggleHUD true)
  (EventDispatchers|AssignPlayerAlive _asbp_player_state (delegate Custom|OnPlayerAlive))
  (EventDispatchers|AssignPlayerDead _asbp_player_state (delegate Custom|OnPlayerDead)))

(event Custom|OnPlayerAlive
  (CallFunction|ToggleHUD true)
  (CallFunction|ToggleSpectate false))

(event Custom|OnPlayerDead
  (params (Instigator :type BP%20Player%20Character%20Object%20Reference) (DeathCauser :type Actor%20Object%20Reference))
  (CallFunction|ToggleHUD false)
  (CallFunction|ToggleSpectate true)
  (if (Variables|/Game/Blueprints/Game/BP_BaseGameState.BP_BaseGameState_C|GetRoundInProgress (.AsBP%20Base%20Game%20State (Utilities|Casting|CastToBP_BaseGameState (Game|GetGameState))))
    (Default|SetDeathInfo (Variables|Default|GetSpectateWidget) Instigator DeathCauser)))

(event Custom|OnRoundEnded
  (params (Reason :type String))
  (CallFunction|ToggleHUD false)
  (CallFunction|ToggleSpectate false)
  (CallFunction|ToggleTap false))

(event EventDrawHUD
  (params (SizeX :type Integer) (SizeY :type Integer))
  ;[1 1 1] Юзать для мобилок
)

(event EventBeginPlay
  (bind _returnvalue (Game|GetGameState))
  (bind _asbp_base_game_state (Utilities|Casting|CastToBP_BaseGameState _returnvalue))
  (EventDispatchers|AssignRoundStarted _asbp_base_game_state (delegate Custom|OnRoundStarted))
  (EventDispatchers|AssignRoundEnded _asbp_base_game_state (delegate Custom|OnRoundEnded)))

(fn ConstructionScript)

(fn ToggleHUD
  (params (Show :type Boolean))
  (if Show
    (if (Variables|/Game/Blueprints/Player/BP_PlayerState.BP_PlayerState_C|GetAlive (.AsBP%20Player%20State (Utilities|Casting|CastToBP_PlayerState (Variables|/Script/Engine.Controller|GetPlayerState (Game|Player|GetOwningPlayerController)))))
      (bind _hudwidget (Variables|Default|GetHUDWidget)
        (:then
          (UserInterface|Viewport|AddtoViewport _hudwidget 0))
        (:else
          (bind _returnvalue (UserInterface|CreateWidget (Variables|Default|GetHUDWidgetClass) (Game|Player|GetOwningPlayerController)))
          (bind _output_get (Variables|Default|SetHUDWidget _returnvalue))
          (UserInterface|Viewport|AddtoViewport _output_get 0))))
    (else
      (bind _hudwidget_2 (Variables|Default|GetHUDWidget)
        (:then
          (Widget|RemovefromParent _hudwidget_2))
        (:else)))))

(fn ToggleTap
  (params (Show :type Boolean))
  (if (Variables|/Game/Blueprints/Game/BP_BaseGameState.BP_BaseGameState_C|GetRoundInProgress (.AsBP%20Base%20Game%20State (Utilities|Casting|CastToBP_BaseGameState (Game|GetGameState))))
    (if false
      (bind _tabwidget (Variables|Default|GetTabWidget)
        (:then
          (UserInterface|Viewport|AddtoViewport _tabwidget 0))
        (:else
          (bind _returnvalue (UserInterface|CreateWidget (Variables|Default|GetTabWidgetClass) (Game|Player|GetOwningPlayerController)))
          (bind _output_get (Variables|Default|SetTabWidget _returnvalue))
          (UserInterface|Viewport|AddtoViewport _output_get 0)))
      (else
        (bind _tabwidget_2 (Variables|Default|GetTabWidget)
          (:then
            (Widget|RemovefromParent _tabwidget_2))
          (:else))))))

(fn ToggleSpectate
  (params (Show :type Boolean))
  (if (Variables|/Game/Blueprints/Game/BP_BaseGameState.BP_BaseGameState_C|GetRoundInProgress (.AsBP%20Base%20Game%20State (Utilities|Casting|CastToBP_BaseGameState (Game|GetGameState))))
    (if false
      (bind _spectatewidget (Variables|Default|GetSpectateWidget)
        (:then
          (UserInterface|Viewport|AddtoViewport _spectatewidget 0))
        (:else
          (bind _returnvalue (UserInterface|CreateWidget (Variables|Default|GetSpectateWidgetClass) (Game|Player|GetOwningPlayerController)))
          (bind _output_get (Variables|Default|SetSpectateWidget _returnvalue))
          (UserInterface|Viewport|AddtoViewport _output_get 0)))
      (else
        (bind _spectatewidget_2 (Variables|Default|GetSpectateWidget)
          (:then
            (Widget|RemovefromParent _spectatewidget_2))
          (:else))))))