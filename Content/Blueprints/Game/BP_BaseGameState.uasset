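; BP_BaseGameState is a base game state that tracks round progress and elapsed round time.
; On the authority, it binds to BP_BaseGamemode's round start and end events to set RoundInProgress, multicasting the end reason.
; The RoundInProgress RepNotify fires RoundStarted and starts or clears an authority-only one-second timer.
; Each tick updates minutes and seconds and calls TimeEnded once the game mode's TimeLimit is reached.
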(event EventBeginPlay
  (Networking|SwitchHasAuthority
    (:Authority
      (|Bindroundend)
      (|BindRoundStart))))

(fn ConstructionScript)

(fn StartRoundTimer
  (bind _returnvalue (Utilities|Time|SetTimerbyFunctionName 0 "RoundTimeTick" 1.0 true))
  (Variables|RoundTime|SetTimeTickTimer _returnvalue))

(fn RoundTimeTick
  (bind _output_get (Variables|RoundTime|SetRoundTime (+ (Variables|RoundTime|GetRoundTime) (Math|Timespan|MakeTimespan 0 0 0 1)))) ; + 1 sec to round time
  (Variables|RoundTime|SetCurrentMinute (.Minutes (Math|Timespan|BreakTimespan _output_get)))
  (Variables|RoundTime|SetCurrentSecond (.Seconds (Math|Timespan|BreakTimespan _output_get)))
  (if (and (>= (Variables|RoundTime|GetRoundTime) (Variables|/Game/Blueprints/Game/BP_BaseGamemode.BP_BaseGamemode_C|GetTimeLimit (.AsBP%20Base%20Gamemode (Utilities|Casting|CastToBP_BaseGamemode (Game|GetGameMode))))) (Variables|Default|GetRoundInProgress)) ; Time limit reachd
    (Default|CallTimeEnded)))

(fn OnRepRoundinProgress
  (if (Variables|Default|GetRoundInProgress)
    (Default|CallRoundStarted)
    (Networking|SwitchHasAuthority
      (:Authority
        (CallFunction|StartRoundTimer)))
    (else
      (Networking|SwitchHasAuthority
        (:Authority
          (Utilities|Time|ClearandInvalidateTimerbyHandle (Variables|RoundTime|GetTimeTickTimer)))))))

(fn GetRoudTime
  (return (Variables|RoundTime|GetCurrentMinute) (Variables|RoundTime|GetCurrentSecond)))

(event Custom|OnRoundStarted
  (Variables|Default|SetRoundInProgress true))

(event Custom|OnRoundEnded
  (params (Reason :type String))
  (CallFunction|Multicast-RoundEnd Reason)
  (Variables|Default|SetRoundInProgress false))

(event Custom|Multicast-RoundEnd
  (params (Reason :type String))
  (Default|CallRoundEnded Reason))