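; BP_Functions_GlobalGetters is a Blueprint function library of shared getters for the game's core framework objects.
; It returns the game mode cast to base or team variants, a controller's player state cast to base or team variants, and a pawn's controller cast to BP_PlayerController.
; IsAnotherTeam compares the Team values on two controllers' team player states to tell whether they are on different teams.
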(fn GetGamemode
  (return (.AsBP%20Base%20Gamemode (Utilities|Casting|CastToBP_BaseGamemode (Game|GetGameMode)))))

(fn GetTeamGamemode
  (return (.AsBP%20Team%20Gamemode (Utilities|Casting|CastToBP_TeamGamemode (Game|GetGameMode)))))

(fn GetPlayerStatebyController
  (params (Controller :type Controller%20Object%20Reference))
  (return (.AsBP%20Player%20State (Utilities|Casting|CastToBP_PlayerState (Variables|/Script/Engine.Controller|GetPlayerState Controller)))))

(fn GetCharactersController
  (params (Pawn :type Pawn%20Object%20Reference))
  (return (.AsBP%20Player%20Controller (Utilities|Casting|CastToBP_PlayerController (Pawn|GetController Pawn)))))

(fn GetTeamPlayerStatebyController
  (params (Controller :type Controller%20Object%20Reference))
  (return (.AsBP%20Team%20Player%20State (Utilities|Casting|CastToBP_TeamPlayerState (Variables|/Script/Engine.Controller|GetPlayerState Controller)))))

(fn IsAnotherTeam
  (params (Player :type Controller%20Object%20Reference) (OtherPlayer :type Controller%20Object%20Reference))
  (return (Utilities|Enum|NotEqual(Enum) (Variables|/Game/Blueprints/Player/BP_TeamPlayerState.BP_TeamPlayerState_C|GetTeam (CallFunction|GetTeamPlayerStatebyController Player)) (Variables|/Game/Blueprints/Player/BP_TeamPlayerState.BP_TeamPlayerState_C|GetTeam (CallFunction|GetTeamPlayerStatebyController OtherPlayer)))))